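; Enemy spawner actor for a twin-stick arena game that adds AI enemies inside a box volume.
; Its SpawnEnemy event counts living EnemyCharacter actors and compares that to EnemyLimit plus a bonus that grows with the game mode's score.
; When under that cap, it spawns one enemy at a random point in SpawnVolume.
; Nothing in this graph calls the event.
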(event Custom|SpawnEnemy
  (bind _spawnvolume (Variables|Default|GetSpawnVolume))
  (bind _outactors (Actor|GetAllActorsOfClass "/Game/Blueprints/EnemyCharacter.EnemyCharacter_C"))
  (bind _astwin_stick_arena_game_mode (Utilities|Casting|CastToTwinStickArenaGameMode (Game|GetGameMode)))
  (if (> (+ (/ (Variables|/Game/Blueprints/TwinStickArenaGameMode.TwinStickArenaGameMode_C|GetScore _astwin_stick_arena_game_mode) 1000) (Variables|Default|GetEnemyLimit)) (Utilities|Array|Length _outactors))
    (AI|SpawnAIFromClass "/Game/Blueprints/EnemyCharacter.EnemyCharacter_C" 0 (Math|Random|RandomPointinBoundingBox (Transformation|GetWorldLocation _spawnvolume) (Components|Box|GetScaledBoxExtent _spawnvolume)) "0, 0, 0" false)))

(event EventBeginPlay)

(event Collision|EventActorBeginOverlap
  (params (OtherActor :type Actor%20Object%20Reference)))

(event EventTick
  (params (DeltaSeconds :type Float%20%28single-precision%29)))

(fn ConstructionScript)