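; Enemy character for a twin-stick arena that damages the hero on a repeating timer while their actors overlap.
; AffectHealth recalculates health; on death it awards score through the game mode, stops colliding with pawns and dynamic objects, detaches its controller, then explodes and destroys itself after a delay.
; The construction script tints the body with EnemyColor through a dynamic material instance.
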(event Custom|DamageHero
  ;[1 1 1] AttackingHero
  (Default|AffectHealth (Variables|Default|Gethero) (Variables|Default|GetDamage)))

(event EventBeginPlay)

(event Collision|EventActorBeginOverlap
  (params (OtherActor :type Actor%20Object%20Reference))
  ;[1 1 1] AttackingHero
  (bind _ashero_character (Utilities|Casting|CastToHeroCharacter OtherActor))
  (Variables|Default|Sethero _ashero_character)
  (Utilities|Time|SetTimerbyFunctionName 0 "DamageHero" (/ 1.0 (Variables|Default|GetAttackPerSecond)) true))

(event EventTick
  (params (DeltaSeconds :type Float%20%28single-precision%29)))

(event EventAffectHealth
  (params (Delta :type Float%20%28single-precision%29))
  (bind _capsulecomponent (Variables|Default|GetCapsuleComponent))
  (Class|BaseCharacter|CalculateHealth Delta)
  (Development|PrintString (Utilities|String|ToString(Float) (Variables|Default|GetHealth)))
  (if (Variables|Default|GetisDead)
    (bind _astwin_stick_arena_game_mode (Utilities|Casting|CastToTwinStickArenaGameMode (Game|GetGameMode)))
    (Default|IncrementScore _astwin_stick_arena_game_mode 500)
    (Collision|SetCollisionResponsetoChannel _capsulecomponent "ECC_WorldDynamic" "ECR_Ignore")
    (Collision|SetCollisionResponsetoChannel _capsulecomponent "ECC_Pawn" "ECR_Ignore")
    (Class|Pawn|DetachfromControllerPendingDestroy)
    (Utilities|FlowControl|Delay 1.9)
    (Game|SpawnActorfromClass "/Game/Blueprints/Explosion.Explosion_C" (Transformation|GetActorTransform) "Undefined" 0 0)
    (Actor|DestroyActor)))

(event Collision|EventActorEndOverlap
  (params (OtherActor :type Actor%20Object%20Reference))
  ;[1 1 1] AttackingHero
  (if (== OtherActor (Variables|Default|Gethero))
    (Utilities|Time|ClearTimerbyFunctionName 0 "DamageHero")))

(fn ConstructionScript
  (bind _returnvalue (Rendering|Material|CreateDynamicMaterialInstance (Variables|Character|GetMesh) 0 0 "None" :!class /Script/Engine.PrimitiveComponent))
  (bind _output_get (Variables|Default|SetDynamyte _returnvalue))
  (Rendering|Material|SetVectorParameterValue _output_get "BodyColor" (Variables|Default|GetEnemyColor) :!class /Script/Engine.MaterialInstanceDynamic))