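; A laser projectile Blueprint that reacts when it overlaps another actor.
; Actors implementing IDamageble that lack the "Friendly" tag receive the projectile's Damage through an interface message, with a laser explosion sound and sparks.
; Other actors implementing ISmallCollision get a separate object-impact sound and sparks.
; Both hit paths destroy the projectile, while friendly damageable actors and all other overlaps leave it intact.
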(event EventBeginPlay)

(event Collision|EventActorBeginOverlap
  (params (OtherActor :type Actor%20Object%20Reference))
  (bind _returnvalue (Transformation|GetActorTransform))
  (bind _lazermesh (Variables|Default|GetLazerMesh))
  (if (Utilities|DoesObjectImplementInterface OtherActor "/Game/Blueprints/iDamageble.iDamageble_C")
    (if (not (Actor|ActorHasTag OtherActor "Friendly"))
      (Class|IDamageble|AffectHealth(Message) OtherActor (Variables|Default|GetDamage))
      (Audio|SpawnSoundAttached "/Game/Music/LaserExplosion.LaserExplosion" _lazermesh "None" "0, 0, 0" "0, 0, 0" "KeepRelativeOffset" false 1.0 1.0 0.0 0 0)
      (Effects|SpawnEmitteratLocation "/Game/Effects/LazerSparks.LazerSparks" (.location _returnvalue) (.rotation _returnvalue) (.scale _returnvalue))
      (Actor|DestroyActor :!label _label))
    (elif (Utilities|DoesObjectImplementInterface OtherActor "/Game/Blueprints/iSmallCollision.iSmallCollision_C")
      (Audio|SpawnSoundAttached "/Game/Music/ObjectExplosion.ObjectExplosion" _lazermesh "None" "0, 0, 0" "0, 0, 0" "KeepRelativeOffset" false 1.0 1.0 0.0 0 0)
      (Effects|SpawnEmitteratLocation "/Game/Effects/LazerSparksObject.LazerSparksObject" (.location _returnvalue) (.rotation _returnvalue) (.scale _returnvalue))
      (goto _label))))

(event EventTick
  (params (DeltaSeconds :type Float%20%28single-precision%29)))

(fn ConstructionScript)